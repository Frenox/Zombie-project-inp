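; BP_Zombie_Idle is a zombie that plays scripted idle animations directly on its mesh.
; After a random start delay on BeginPlay, the Anim variable selects a get-up-to-scream, prone-to-stand, standing idle or looping crawl.
; All but the crawl end in RandomGrab, a self-calling event that repeats the idle and occasionally inserts an attack animation.
; Sequencing relies on fixed Delays.
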(event `self.ReceiveBeginPlay`
  (bind _mesh (`self.Mesh`))
  ;[1 1 1] Start animations
  (`parent.ReceiveBeginPlay`)
  (`KismetSystemLibrary.Delay` (`KismetMathLibrary.RandomFloatInRange` 0.0 5.0))
  (switch `int` (`self.Anim`)
    (:`Default`
      (`SkeletalMeshComponent.PlayAnimation` _mesh "/Game/BSP_ZombieAnims/Animations/GetUp/AM_NAAT_Human_ZombieGetUpToScream.AM_NAAT_Human_ZombieGetUpToScream" false)
      (`KismetSystemLibrary.Delay` 10.0)
      (`SkeletalMeshComponent.PlayAnimation` _mesh "/Game/BSP_ZombieAnims/Animations/Standing/AS_NAAT_Zombie_BL_Idle.AS_NAAT_Zombie_BL_Idle" false :!label _label)
      (`self.RandomGrab` :!label _label_2))
    (:`0`
      (`SkeletalMeshComponent.PlayAnimation` _mesh "/Game/BSP_ZombieAnims/Animations/GetUp/AS_NAAT_Zombie_LieProne_To_Idle_Stand.AS_NAAT_Zombie_LieProne_To_Idle_Stand" false)
      (`KismetSystemLibrary.Delay` 10.13)
      (goto _label))
    (:`1`
      (`SkeletalMeshComponent.PlayAnimation` _mesh "/Game/BSP_ZombieAnims/Animations/Standing/AS_NAAT_Zombie_BL_Idle.AS_NAAT_Zombie_BL_Idle" false)
      (`KismetSystemLibrary.Delay` 6.63)
      (goto _label_2))
    (:`2`
      (`SkeletalMeshComponent.PlayAnimation` _mesh "/Game/BSP_ZombieAnims/Animations/Crawl/AS_NAAT_Zombie_Crawl_Idle.AS_NAAT_Zombie_Crawl_Idle" true))))

(event `RandomGrab`
  (bind _returnvalue (`KismetMathLibrary.RandomIntegerInRange` 0 15))
  (if (or (== _returnvalue 4) (== _returnvalue 7))
    (`SkeletalMeshComponent.PlayAnimation` (`self.Mesh`) "/Game/BSP_ZombieAnims/Animations/Standing/Attack/AS_NAAT_Zombie_Attack_BH_Stand.AS_NAAT_Zombie_Attack_BH_Stand" false)
    (`KismetSystemLibrary.Delay` 1.93)
    (`SkeletalMeshComponent.PlayAnimation` (`self.Mesh`) "/Game/BSP_ZombieAnims/Animations/Standing/AS_NAAT_Zombie_BL_Idle.AS_NAAT_Zombie_BL_Idle" false)
    (`KismetSystemLibrary.Delay` 6.63)
    (`self.RandomGrab`)
    (else
      (`SkeletalMeshComponent.PlayAnimation` (`self.Mesh`) "/Game/BSP_ZombieAnims/Animations/Standing/AS_NAAT_Zombie_BL_Idle.AS_NAAT_Zombie_BL_Idle" false)
      (`KismetSystemLibrary.Delay` 6.63)
      (`self.RandomGrab`))))

(fn `UserConstructionScript`
  (`parent.UserConstructionScript`))