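; BP_VideoHandler drives video-based story branches, looking up the current video by Id in the DATA_Videos table.
; VideoStarted stores the Id, prints the row's Ref and waits a fixed delay in place of playback before firing VideoEnded.
; VideoEnded reads the row's Surviving flag and branches to MakeChoice or Death, both currently placeholder print-string events.
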(event `VideoStarted`
  (params (Id :type Name))
  (bind _output_get (set `self.currentVideoId` Id))
  (bind _returnvalue (`|GetDataTableRow` "/Game/Videos_Data/DataTable/DATA_Videos.DATA_Videos" _output_get)
    (:`then`
      (`KismetSystemLibrary.PrintString` (break `/Game/Videos_Data/DataTable/STRUCT_Videos` _returnvalue))
      (`KismetSystemLibrary.Delay` 5.0)
      (`self.VideoEnded`))))

(event `VideoEnded`
  (bind _returnvalue (`|GetDataTableRow` "/Game/Videos_Data/DataTable/DATA_Videos.DATA_Videos" (`self.currentVideoId`))
    (:`then`
      (if (`.Surviving_11_4E4C353E4E6F83B9C0B3D1A327845D79` (break `/Game/Videos_Data/DataTable/STRUCT_Videos` _returnvalue))
        (`self.MakeChoice`)
        (else
          (`self.Death`))))))

(event `MakeChoice`
  (`KismetSystemLibrary.PrintString` "Choice event"))

(event `Death`
  (`KismetSystemLibrary.PrintString` "Died"))

(fn `UserConstructionScript`)