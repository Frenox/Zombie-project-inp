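; BP_Screen is a video screen actor that plays clips by ID and moves between a fixed playback position and a lower reset position.
; videoStart opens the source from the DATA_Videos row on a MediaPlayer, then raises the screen after a brief delay.
; It then waits on GetVideoDuration and notifies the BP_VideoHandler found at BeginPlay, using a timed delay rather than a media-end event.
; ResetPosition drops the screen back down.
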(event `self.ReceiveBeginPlay`
  (bind _returnvalue (`GameplayStatics.GetActorOfClass` "/Game/BP_VideoHandler.BP_VideoHandler_C"))
  (set `self.videoHandler` _returnvalue))

(event `videoStart`
  (params (videoID :type Name))
  (bind (_returnvalue_days _returnvalue_hours _returnvalue_minutes _returnvalue_seconds _returnvalue_milliseconds) (`KismetMathLibrary.BreakTimespan` (`MediaPlayer.GetDuration` (`self.mediaPlayer`))))
  (bind _returnvalue (`|GetDataTableRow` "/Game/Videos_Data/DataTable/DATA_Videos.DATA_Videos" videoID)
    (:`then`
      (`MediaPlayer.OpenSource` (`self.mediaPlayer`) (break `/Game/Videos_Data/DataTable/STRUCT_Videos` _returnvalue))
      (`KismetSystemLibrary.Delay` 0.2)
      (if (not (== (`self.K2_GetActorLocation`) (-110.0 0.0 172.0)))
        (`self.K2_SetActorLocation` (-110.0 0.0 172.0)))
      (`KismetSystemLibrary.Delay` (+ (* 60 (`KismetMathLibrary.Conv_IntToDouble` _returnvalue_minutes)) (`KismetMathLibrary.Conv_IntToDouble` _returnvalue_seconds) (/ (`KismetMathLibrary.Conv_IntToDouble` _returnvalue_milliseconds) 1000.0)))
      (`/Game/BP_VideoHandler.VideoEnded` (`self.videoHandler`)))))

(event `ResetPosition`
  (`self.K2_SetActorLocation` (-110.0 0.0 -115.0)))

(fn `UserConstructionScript`)